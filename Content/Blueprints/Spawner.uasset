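; Spawner actor that scatters a configurable number of actors, apparently NPCs, within a radius around itself when its Generator event runs.
; Each spawn rotates the forward vector by a random yaw and scales it by the square root of a random squared radius, giving uniform disc distribution.
; Spawns are raised slightly and given random facing.
; The construction script sizes a sphere component to match the radius.
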(event Custom|Generator
  (for _index (range 0 (- (Variables|Default|GetNPCCount) 1))
    (Game|SpawnActorfromClass "/Game/ThirdPersonBP/Blueprints/ThirdPersonCharacter.ThirdPersonCharacter_C" (Math|Transform|MakeTransform (+ (+ (* (Math|Vector|RotateVector (Transformation|GetActorForwardVector) (Math|Rotator|MakeRotator 0.0 0.0 (Math|Random|RandomFloatinRange 0.0 3.6e+02))) (Math|Float|Sqrt (Math|Random|RandomFloatinRange 0.0 (* (Variables|Default|GetRadius) (Variables|Default|GetRadius))))) (Transformation|GetActorLocation)) "0, 0,100.000000") (Math|Rotator|MakeRotator 0.0 0.0 (Math|Random|RandomFloatinRange 0.0 3.6e+02)) "1,1,1") "Undefined" 0 0)))

(fn ConstructionScript
  (Components|Sphere|SetSphereRadius (Variables|Default|GetSphere) (Variables|Default|GetRadius) true))